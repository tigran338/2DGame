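; BP_BadMushroom is an interactive mushroom that hurts the BP_Ninja player and destroys itself when the interaction key is active.
; Its Box overlap events set an overlap flag and store the ninja, and Tick polls that ninja's InteractionKey before applying DamageAmount.
; Tick forces the flag true and the stored reference is never cleared, so the interaction still fires after the ninja leaves the box.
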(event OnComponentBeginOverlap(Box)
  (params (OverlappedComponent :type Primitive%20Component%20Object%20Reference) (OtherActor :type Actor%20Object%20Reference) (OtherComp :type Primitive%20Component%20Object%20Reference) (OtherBodyIndex :type Integer) (bFromSweep :type Boolean) (SweepResult :type Hit%20Result%20Structure%20%28by%20ref%29))
  (Utilities|Casting|CastToBP_Ninja OtherActor)
  (Variables|Default|SetIsOverlaping true)
  (Variables|Default|SetActorOverlaping OtherActor))

(event OnComponentEndOverlap(Box)
  (params (OverlappedComponent :type Primitive%20Component%20Object%20Reference) (OtherActor :type Actor%20Object%20Reference) (OtherComp :type Primitive%20Component%20Object%20Reference) (OtherBodyIndex :type Integer))
  (Utilities|Casting|CastToBP_Ninja OtherActor)
  (Variables|Default|SetIsOverlaping false))

(event EventBeginPlay)

(event Collision|EventActorBeginOverlap
  (params (OtherActor :type Actor%20Object%20Reference)))

(event EventTick
  (params (DeltaSeconds :type Float%20%28single-precision%29))
  (Variables|Default|SetIsOverlaping true)
  (if true
    (bind _asbp_ninja (Utilities|Casting|CastToBP_Ninja (Variables|Default|GetActorOverlaping)))
    (if (Variables|/Game/BP/Character/BP_Ninja.BP_Ninja_C|GetInteractionKey _asbp_ninja)
      (Default|Hurt _asbp_ninja (Variables|Default|GetDamage%20Amount))
      (Actor|DestroyActor))))

(fn ConstructionScript)
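; BP_Spider is a flipbook-animated enemy that chases BP_Ninja along the X axis while the player is inside its detection sphere.
; Sphere overlaps toggle FoundPC and the walk/idle flipbooks, while Tick drives movement and control-rotation facing from relative player position.
; spiderHurt subtracts DmgTaken and briefly pauses animation, while capsule contact with the ninja zeroes health.
; Tick destroys the spider only when health equals exactly zero.
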(event OnComponentBeginOverlap(Sphere)
  (params (OverlappedComponent :type Primitive%20Component%20Object%20Reference) (OtherActor :type Actor%20Object%20Reference) (OtherComp :type Primitive%20Component%20Object%20Reference) (OtherBodyIndex :type Integer) (bFromSweep :type Boolean) (SweepResult :type Hit%20Result%20Structure%20%28by%20ref%29))
  ;[0.875 0.6301 1] Movement + Rotation
  ;;[1 1 1] Overlap w/ PC
  (Utilities|Casting|CastToBP_Ninja OtherActor)
  (Variables|Default|SetfoundPC true)
  (Sprite|SetFlipbook (Variables|Default|GetSprite) "/Game/BP/Enemies/Spider/Flipbook/spider_walk.spider_walk"))

(event OnComponentEndOverlap(Sphere)
  (params (OverlappedComponent :type Primitive%20Component%20Object%20Reference) (OtherActor :type Actor%20Object%20Reference) (OtherComp :type Primitive%20Component%20Object%20Reference) (OtherBodyIndex :type Integer))
  ;[0.875 0.6301 1] Movement + Rotation
  ;;[1 1 1] Overlap w/ PC
  (Utilities|Casting|CastToBP_Ninja OtherActor)
  (Variables|Default|SetfoundPC false)
  (Sprite|SetFlipbook (Variables|Default|GetSprite) "/Game/BP/Enemies/Spider/Flipbook/spider_idle.spider_idle"))

(event OnComponentBeginOverlap(CapsuleComponent)
  (params (OverlappedComponent :type Primitive%20Component%20Object%20Reference) (OtherActor :type Actor%20Object%20Reference) (OtherComp :type Primitive%20Component%20Object%20Reference) (OtherBodyIndex :type Integer) (bFromSweep :type Boolean) (SweepResult :type Hit%20Result%20Structure%20%28by%20ref%29))
  (Utilities|Casting|CastToBP_Ninja OtherActor)
  (Variables|Default|SetcurrHealth 0.0))

(event Custom|spiderHurt
  (bind _sprite (Variables|Default|GetSprite))
  (Utilities|FlowControl|Sequence
    (:then_0
      (Variables|Default|SetcurrHealth (- (Variables|Default|GetcurrHealth) (Variables|Default|GetdmgTaken))))
    (:then_1
      (Audio|Components|Audio|Stop _sprite)
      (Utilities|FlowControl|Delay 0.5)
      (Audio|Components|Audio|Play _sprite))))

(event Custom|movrit
  (params (AxisVal :type Float%20%28double-precision%29))
  (bind _returnvalue (Pawn|GetController))
  ;[0.875 0.6301 1] Movement + Rotation
  ;;[1 1 1] Rotate + move
  (Pawn|Input|AddMovementInput "1.000000, 0, 0" AxisVal false)
  (Math|Float|CompareFloat AxisVal 0.0
    (:>
      (Pawn|SetControlRotation _returnvalue (Math|Rotator|MakeRotator 0.0 0.0 0.0)))
    (:<
      (Pawn|SetControlRotation _returnvalue (Math|Rotator|MakeRotator 0.0 0.0 1.8e+02)))))

(event Custom|ai%20follow
  ;[0.875 0.6301 1] Movement + Rotation
  ;;[1 1 1] getPCPos
  (if (Variables|Default|GetfoundPC)
    (bind _asbp_ninja (Utilities|Casting|CastToBP_Ninja (Game|GetPlayerCharacter 0)))
    (Math|Float|CompareFloat (- (.x (Transformation|GetWorldLocation (Variables|Collision|GetCapsuleComponent))) (.x (Transformation|GetWorldLocation (Variables|/Script/Engine.Character|GetCapsuleComponent _asbp_ninja)))) 0.0
      (:>
        (CallFunction|Movrit -0.5))
      (:==
        (CallFunction|Movrit 0.0))
      (:<
        (CallFunction|Movrit 0.5)))))

(event EventTick
  (params (DeltaSeconds :type Float%20%28single-precision%29))
  ;[1 1 1] AI begin code
  (CallFunction|AiFollow)
  (if (== (Variables|Default|GetcurrHealth) 0.0)
    (Actor|DestroyActor)))

(fn ConstructionScript)
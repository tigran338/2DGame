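; BP_Zombie is an enemy that alternates facing along the X axis and destroys itself when its capsule overlaps BP_Ninja.
; A looping timer started on BeginPlay flips IsMoveRight, applying one movement input per tick and snapping control yaw to match the direction.
; The overlap clears that timer after calling DestroyActor.
; A ZombTimer debug counter is left unconnected.
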(event OnComponentBeginOverlap(CapsuleComponent)
  (params (OverlappedComponent :type Primitive%20Component%20Object%20Reference) (OtherActor :type Actor%20Object%20Reference) (OtherComp :type Primitive%20Component%20Object%20Reference) (OtherBodyIndex :type Integer) (bFromSweep :type Boolean) (SweepResult :type Hit%20Result%20Structure%20%28by%20ref%29))
  (Utilities|Casting|CastToBP_Ninja OtherActor)
  (Actor|DestroyActor)
  (CallFunction|EndTimer))

(event Custom|beginCount
  (bind _returnvalue (Utilities|Time|SetTimerbyEvent (delegate Custom|count) 2.0 true)))

(event Custom|endTimer
  (Utilities|Time|ClearandInvalidateTimerbyHandle (stale Custom|beginCount _returnvalue)))

(event Custom|count
  (if (Variables|Default|GetisMoveRight)
    (CallFunction|Movin 1.0)
    (Variables|Default|SetisMoveRight false)
    (else
      (CallFunction|Movin -1.0)
      (Variables|Default|SetisMoveRight true))))

(event Custom|movin
  (params (axisVal :type Float%20%28double-precision%29))
  (bind _returnvalue (Pawn|GetController))
  (Pawn|Input|AddMovementInput "100.000000,0.000000, 0" axisVal false)
  (Math|Float|CompareFloat axisVal 0.0
    (:>
      (Pawn|SetControlRotation _returnvalue (Math|Rotator|MakeRotator 0.0 0.0 0.0)))
    (:<
      (Pawn|SetControlRotation _returnvalue (Math|Rotator|MakeRotator 0.0 0.0 1.8e+02)))))

(event EventBeginPlay
  (CallFunction|BeginCount))

(fn ConstructionScript)
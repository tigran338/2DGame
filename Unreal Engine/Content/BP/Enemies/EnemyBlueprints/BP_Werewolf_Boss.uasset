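; Werewolf boss using flipbook sprites, with a wandering first stage and a player-following stage after dropping to half health.
; Tick picks the stage's movement; TakeDmg advances the stage and, after a delay, resets capsule collision to Pawn.
; BossTimer modulo checks trigger idle stops that disable movement.
; The resume check tests constant 0, so it always passes, flipping patrol direction on every non-stop tick, and "move" sets movement mode None.
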(event Custom|werewolfBossStop
  ;[1 1 1] Werewolf disable/enable movement + set the flipbook to the correct animation
  (Sprite|SetFlipbook (Variables|Default|GetSprite) "/Game/BP/Enemies/AllEnemies/wereWolf_Boss/Flipbooks/wolf-idle.wolf-idle")
  (Pawn|Components|CharacterMovement|DisableMovement (Variables|Character|GetCharacterMovement)))

(event Custom|werewolfBossMove
  ;[1 1 1] Werewolf disable/enable movement + set the flipbook to the correct animation
  (Sprite|SetFlipbook (Variables|Default|GetSprite) "/Game/BP/Enemies/AllEnemies/wereWolf_Boss/Flipbooks/werewolf-running.werewolf-running")
  (Pawn|Components|CharacterMovement|SetMovementMode (Variables|Character|GetCharacterMovement) "MOVE_None" 0))

(event Custom|werewolfBossMoveNotFollow
  (params (move_speed :type Float%20%28double-precision%29))
  ;[1 1 1] Werewolf Moves without following PC
  (if (Variables|Default|GetisMoveRight)
    (CallFunction|BossMoveRot move_speed)
    (else
      (CallFunction|BossMoveRot (* move_speed -1.0))))
  (CallFunction|AddtoBossTimer)
  (if (== (Math|Integer|%(Integer) (Variables|Default|GetbossTimer) 200) 0)
    (CallFunction|WerewolfBossStop)
    (elif (== (Math|Integer|%(Integer) 0 300) 0)
      (Variables|Default|SetisMoveRight (not (Variables|Default|GetisMoveRight)))
      (CallFunction|WerewolfBossMove))))

(event Custom|werewolfAlive
  ;[1 1 1] Werewolf will act according to its stage
  (if (== (Variables|Default|GetbossStage) 0)
    (CallFunction|WerewolfBossMoveNotFollow 1.0)
    (else
      (CallFunction|BossFollowPC 0.75))))

(event EventBeginPlay
  (|CallParentFunction) ; This node is disabled and will not be called.\nDrag off pins to build functionality.
)

(event Collision|EventActorBeginOverlap
  (params (OtherActor :type Actor%20Object%20Reference))
  (|CallParentFunction OtherActor) ; This node is disabled and will not be called.\nDrag off pins to build functionality.
)

(event EventTick
  (params (DeltaSeconds :type Float%20%28single-precision%29))
  (|CallParentFunction DeltaSeconds)
  (CallFunction|WerewolfAlive))

(event EventTakeDmg
  (params (dmgTaken :type Float%20%28double-precision%29))
  ;[0.8706 0.6314 1] Boss will change stages after hitting half health
  (|CallParentFunction dmgTaken)
  (if (and (<= (Variables|Default|GetcurrentHealth) 2e+02) (== (Variables|Default|GetbossStage) 0))
    (CallFunction|NextBossStage)
    (Utilities|FlowControl|Delay 1.5)
    (CallFunction|BossMoveRot 0.1)
    (Collision|SetCollisionProfileName (Variables|Default|GetCapsuleComponent) "Pawn" true :!class /Script/Engine.PrimitiveComponent)))

(event EventBossFollowPC
  (params (Boss%20movement%20speed :type Float%20%28double-precision%29))
  ;[1 1 1] Werewolf follows PC with break after certain time has passed
  (|CallParentFunction Boss%20movement%20speed)
  (if (== (Math|Integer|%(Integer) (Variables|Default|GetbossTimer) 200) 0)
    (CallFunction|WerewolfBossStop)
    (elif (== (Math|Integer|%(Integer) 0 300) 0)
      (CallFunction|WerewolfBossMove)
      (CallFunction|BossMoveRot Boss%20movement%20speed))))

(fn ConstructionScript
  (|CallParentFunction))
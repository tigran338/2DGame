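; Inheritable base Blueprint for bosses, providing shared movement, player detection, timer and stage logic on top of a parent enemy class.
; DetectPC overlaps toggle FoundPC, letting bossFollowPC compare X positions and move toward the player along X, snapping control yaw to face travel direction.
; Each follow move increments BossTimer, while nextBossStage resets it and advances BossStage.
; Damage passes through to the parent enemy logic.
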(event OnComponentBeginOverlap(DetectPC)
  (params (OverlappedComponent :type Primitive%20Component%20Object%20Reference) (OtherActor :type Actor%20Object%20Reference) (OtherComp :type Primitive%20Component%20Object%20Reference) (OtherBodyIndex :type Integer) (bFromSweep :type Boolean) (SweepResult :type Hit%20Result%20Structure%20%28by%20ref%29))
  ;[0.8706 0.6314 1] Logic for all bosses
  ;;[1 1 1] Setting FoundPC for Boss
  (Utilities|Casting|CastToBP_MainCharacter OtherActor)
  (Variables|Default|SetfoundPC true))

(event OnComponentEndOverlap(DetectPC)
  (params (OverlappedComponent :type Primitive%20Component%20Object%20Reference) (OtherActor :type Actor%20Object%20Reference) (OtherComp :type Primitive%20Component%20Object%20Reference) (OtherBodyIndex :type Integer))
  ;[0.8706 0.6314 1] Logic for all bosses
  ;;[1 1 1] Setting FoundPC for Boss
  (Utilities|Casting|CastToBP_MainCharacter OtherActor)
  (Variables|Default|SetfoundPC false))

(event Custom|bossMoveRot
  (params (axis%20Val :type Float%20%28double-precision%29))
  (bind _returnvalue (Pawn|GetController))
  ;[0.8706 0.6314 1] Logic for all bosses
  ;;[1 1 1] Boss Moving/Rotating
  (Pawn|Input|AddMovementInput "1.000000, 0, 0" axis%20Val false)
  (Math|Float|CompareFloat axis%20Val 0.0
    (:>
      (Pawn|SetControlRotation _returnvalue (Math|Rotator|MakeRotator 0.0 0.0 0.0)))
    (:<
      (Pawn|SetControlRotation _returnvalue (Math|Rotator|MakeRotator 0.0 0.0 1.8e+02)))))

(event Custom|bossFollowPC
  (params (Boss%20movement%20speed :type Float%20%28double-precision%29))
  ;[0.8706 0.6314 1] Logic for all bosses
  ;;[1 1 1] Boss Follow Enemy
  (if (Variables|Default|GetfoundPC)
    (bind _asbp_main_character (Utilities|Casting|CastToBP_MainCharacter (Game|GetPlayerCharacter 0)))
    (Math|Float|CompareFloat (- (.x (Transformation|GetWorldLocation (Variables|Default|GetCapsuleComponent))) (.x (Transformation|GetWorldLocation (Variables|/Script/Engine.Actor|GetRootComponent _asbp_main_character)))) 0.0
      (:>
        (CallFunction|BossMoveRot (* Boss%20movement%20speed -1.0)))
      (:<
        (CallFunction|BossMoveRot Boss%20movement%20speed)))
    (CallFunction|AddtoBossTimer)))

(event Custom|addToBossTimer
  ;[0.8706 0.6314 1] Logic for all bosses
  ;;[1 1 1] Update Boss Timer
  (bind _result (Math|Integer|IncrementInt (Variables|Default|GetbossTimer))
    (:%20%20
      (bind _output_get (Variables|Default|SetbossTimer _result))
      (Development|PrintString (Utilities|String|ToString(Integer) _output_get)))))

(event Custom|nextBossStage
  ;[0.8706 0.6314 1] Logic for all bosses
  ;;[1 1 1] Reset timer and then increment boss stage
  (Variables|Default|SetbossTimer 0)
  (bind _result (Math|Integer|IncrementInt (Variables|Default|GetbossStage))
    (:%20%20
      (Variables|Default|SetbossStage _result)
      (Development|PrintString "next boss stage"))))

(event EventBeginPlay)

(event Collision|EventActorBeginOverlap
  (params (OtherActor :type Actor%20Object%20Reference)))

(event EventTick
  (params (DeltaSeconds :type Float%20%28single-precision%29)))

(event EventTakeDmg
  (params (dmgTaken :type Float%20%28double-precision%29))
  ;[0.8706 0.6314 1] Logic for all bosses
  ;;[1 1 1] Boss takes damage just like any other enemy
  (|CallParentFunction dmgTaken))

(fn ConstructionScript
  (|CallParentFunction))
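; BP_Spider1 is a 2D flipbook spider enemy that chases the player character along the X axis.
; A detection sphere toggles the chase flag and swaps between walk and idle flipbooks.
; While chasing, Tick compares X positions to drive quarter-scale movement input toward the player and flips control yaw to face the travel direction.
; An attack box only prints debug text on overlap, with no damage logic.
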(event OnComponentBeginOverlap(SphereColl)
  (params (OverlappedComponent :type Primitive%20Component%20Object%20Reference) (OtherActor :type Actor%20Object%20Reference) (OtherComp :type Primitive%20Component%20Object%20Reference) (OtherBodyIndex :type Integer) (bFromSweep :type Boolean) (SweepResult :type Hit%20Result%20Structure%20%28by%20ref%29))
  ;[0.8706 0.6314 1] Spider AI Follows the PC
  ;;[1 1 1] PC within sphere sets foundPC and flipbook
  (Utilities|Casting|CastToBP_MainCharacter OtherActor)
  (Variables|Default|SetfoundPC true)
  (Sprite|SetFlipbook (Variables|Default|GetSprite) "/Game/BP/Enemies/AllEnemies/Spider/Flipbook/spider_walk.spider_walk"))

(event OnComponentEndOverlap(SphereColl)
  (params (OverlappedComponent :type Primitive%20Component%20Object%20Reference) (OtherActor :type Actor%20Object%20Reference) (OtherComp :type Primitive%20Component%20Object%20Reference) (OtherBodyIndex :type Integer))
  ;[0.8706 0.6314 1] Spider AI Follows the PC
  ;;[1 1 1] PC within sphere sets foundPC and flipbook
  (Utilities|Casting|CastToBP_MainCharacter OtherActor)
  (Variables|Default|SetfoundPC false)
  (Sprite|SetFlipbook (Variables|Default|GetSprite) "/Game/BP/Enemies/AllEnemies/Spider/Flipbook/spider_idle.spider_idle"))

(event OnComponentBeginOverlap(Box)
  (params (OverlappedComponent :type Primitive%20Component%20Object%20Reference) (OtherActor :type Actor%20Object%20Reference) (OtherComp :type Primitive%20Component%20Object%20Reference) (OtherBodyIndex :type Integer) (bFromSweep :type Boolean) (SweepResult :type Hit%20Result%20Structure%20%28by%20ref%29))
  (Utilities|Casting|CastToBP_MainCharacter OtherActor)
  (Development|PrintString "attack!"))

(event OnComponentEndOverlap(Box)
  (params (OverlappedComponent :type Primitive%20Component%20Object%20Reference) (OtherActor :type Actor%20Object%20Reference) (OtherComp :type Primitive%20Component%20Object%20Reference) (OtherBodyIndex :type Integer))
  (Utilities|Casting|CastToBP_MainCharacter OtherActor)
  (Development|PrintString "no"))

(event Custom|spidFollowPC
  ;[0.8706 0.6314 1] Spider AI Follows the PC
  ;;[1 1 1] spider followPC
  (if (Variables|Default|GetfoundPC)
    (bind _asbp_main_character (Utilities|Casting|CastToBP_MainCharacter (Game|GetPlayerCharacter 0)))
    (Math|Float|CompareFloat (- (.x (Transformation|GetWorldLocation (Variables|Default|GetCapsuleComponent))) (.x (Transformation|GetWorldLocation (Variables|/Script/Engine.Actor|GetRootComponent _asbp_main_character)))) 0.0
      (:>
        (CallFunction|SpidMoveRot -0.25))
      (:==
        (CallFunction|SpidMoveRot 0.0))
      (:<
        (CallFunction|SpidMoveRot 0.25)))))

(event Custom|spidMoveRot
  (params (axisValue :type Float%20%28double-precision%29))
  (bind _returnvalue (Pawn|GetController))
  ;[0.8706 0.6314 1] Spider AI Follows the PC
  ;;[1 1 1] Spider movement and rotation
  (Pawn|Input|AddMovementInput "1.000000, 0, 0" axisValue false)
  (Math|Float|CompareFloat axisValue 0.0
    (:>
      (Pawn|SetControlRotation _returnvalue (Math|Rotator|MakeRotator 0.0 0.0 0.0)))
    (:<
      (Pawn|SetControlRotation _returnvalue (Math|Rotator|MakeRotator 0.0 0.0 1.8e+02)))))

(event EventBeginPlay)

(event EventTick
  (params (DeltaSeconds :type Float%20%28single-precision%29))
  (CallFunction|SpidFollowPC))

(fn ConstructionScript
  (|CallParentFunction))
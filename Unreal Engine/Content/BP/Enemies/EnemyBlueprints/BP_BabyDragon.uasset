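; BP_BabyDragon is a flying enemy that patrols back and forth and hurts the player on contact.
; Tick drives movement input along its fly-speed vector, snaps control yaw to face the travel direction, and increments a counter that flips direction every 200 frames, so patrol timing is frame-based.
; HitBox overlap calls Hurt on BP_MainCharacter only when the overlapping component is that character's capsule.
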(event OnComponentBeginOverlap(HitBox)
  (params (OverlappedComponent :type Primitive%20Component%20Object%20Reference) (OtherActor :type Actor%20Object%20Reference) (OtherComp :type Primitive%20Component%20Object%20Reference) (OtherBodyIndex :type Integer) (bFromSweep :type Boolean) (SweepResult :type Hit%20Result%20Structure%20%28by%20ref%29))
  ;[1 1 1] Dmg Player
  (bind _asbp_main_character (Utilities|Casting|CastToBP_MainCharacter OtherActor))
  (if (== (Variables|/Script/Engine.Character|GetCapsuleComponent _asbp_main_character) OtherComp)
    (Default|Hurt _asbp_main_character 0.2 1)))

(event Custom|babyDragBackAndForth
  ;[0.8745 0.6314 1] Baby Dragon movement and Rotation
  ;;[1 1 1] Direction switch for Baby Dragon
  (if (Variables|Default|GetisMoveRight)
    (CallFunction|BabyDragMoveRot 0.25)
    (else
      (CallFunction|BabyDragMoveRot -0.25)))
  (bind _result (Math|Integer|IncrementInt (Variables|Default|GetbabyDragTimer))
    (:%20%20
      (bind _output_get (Variables|Default|SetbabyDragTimer _result))
      (if (== (Math|Integer|%(Integer) _output_get 200) 0)
        (Variables|Default|SetisMoveRight (not (Variables|Default|GetisMoveRight)))))))

(event Custom|babyDragMoveRot
  (params (Axis%20Val :type Float%20%28double-precision%29))
  (bind _returnvalue (Pawn|GetController))
  ;[0.8745 0.6314 1] Baby Dragon movement and Rotation
  ;;[1 1 1] Movement and Rotation for baby Dragon
  (Pawn|Input|AddMovementInput (Math|Vector|MakeVector (Variables|Default|GetbabydragFlySpeed) 0.0 0.0) Axis%20Val false)
  (Math|Float|CompareFloat Axis%20Val 0.0
    (:>
      (Pawn|SetControlRotation _returnvalue (Math|Rotator|MakeRotator 0.0 0.0 0.0)))
    (:<
      (Pawn|SetControlRotation _returnvalue (Math|Rotator|MakeRotator 0.0 0.0 1.8e+02)))))

(event EventBeginPlay)

(event Collision|EventActorBeginOverlap
  (params (OtherActor :type Actor%20Object%20Reference)))

(event EventTick
  (params (DeltaSeconds :type Float%20%28single-precision%29))
  (CallFunction|BabyDragBackandForth))

(fn ConstructionScript
  (|CallParentFunction))
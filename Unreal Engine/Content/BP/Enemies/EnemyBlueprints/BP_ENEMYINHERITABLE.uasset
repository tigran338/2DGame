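; Base enemy Blueprint, apparently meant for inheritance, that handles damage, stun and death for a flipbook-animated character.
; The takeDmg event subtracts health, flags the enemy as hurt, and pauses its sprite and movement for StunTime before restoring walking.
; A Sequence checks health during that stun, stopping the enemy at zero or below and destroying it after a second, without cancelling the stun recovery.
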(event Custom|takeDmg
  (params (dmgTaken :type Float%20%28double-precision%29))
  (bind _sprite (Variables|Default|GetSprite))
  (bind _charactermovement (Variables|Character|GetCharacterMovement))
  ;[0.8745 0.6314 1] Damage Logic
  (Utilities|FlowControl|Sequence
    (:then_0
      ;;[1 1 1] Decrease Health, disable movement/stun. then after stun, continue as before
      (Variables|Default|SetcurrentHealth (- (Variables|Default|GetcurrentHealth) dmgTaken))
      (Variables|Default|SetisHurt true)
      (Audio|Components|Audio|Stop _sprite)
      (Pawn|Components|CharacterMovement|DisableMovement _charactermovement)
      (Utilities|FlowControl|Delay (Variables|Default|GetstunTime))
      (Audio|Components|Audio|Play _sprite)
      (Variables|Default|SetisHurt false)
      (Pawn|Components|CharacterMovement|SetMovementMode _charactermovement "MOVE_Walking" 0)
      (Development|PrintString "dmg taken"))
    (:then_1
      ;;[1 1 1] Death handling: if current Health == 0, then stop flipbook & movement. then after 1 second will destroy the actor
      (if (<= (Variables|Default|GetcurrentHealth) 0.0)
        (Audio|Components|Audio|Stop _sprite)
        (Pawn|Components|CharacterMovement|DisableMovement _charactermovement)
        (Utilities|FlowControl|Delay 1.0)
        (Actor|DestroyActor)
        (Development|PrintString "dead")))))

(fn ConstructionScript)
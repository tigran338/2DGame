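; Ghost enemy for a side-scrolling level that patrols back and forth along world X and hurts the main character on contact.
; Tick drives movement input and flips control yaw, reversing direction on a game-time timer, with starting direction read from the sprite's yaw.
; HitBox overlap with the character's capsule calls Hurt.
; A PuffEffect helper spawns an effect actor at the ghost's capsule, nudged along Y.
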(event OnComponentBeginOverlap(HitBox)
  (params (OverlappedComponent :type Primitive%20Component%20Object%20Reference) (OtherActor :type Actor%20Object%20Reference) (OtherComp :type Primitive%20Component%20Object%20Reference) (OtherBodyIndex :type Integer) (bFromSweep :type Boolean) (SweepResult :type Hit%20Result%20Structure%20%28by%20ref%29))
  (bind _asbp_main_character (Utilities|Casting|CastToBP_MainCharacter OtherActor))
  (if (== (Variables|/Script/Engine.Character|GetCapsuleComponent _asbp_main_character) OtherComp)
    (Default|Hurt _asbp_main_character 0.2 1)))

(event Custom|zombMoveRot
  (params (axisVal :type Float%20%28double-precision%29))
  (bind _returnvalue (Pawn|GetController))
  ;[0.8745 0.6314 1] Zombie Movement and Rotation Logic
  ;;[1 1 1] Movement + rotation for zombie
  (Pawn|Input|AddMovementInput "1.000000,0.000000, 0" axisVal false)
  (Math|Float|CompareFloat axisVal 0.0
    (:>
      (Pawn|SetControlRotation _returnvalue (Math|Rotator|MakeRotator 0.0 0.0 0.0)))
    (:<
      (Pawn|SetControlRotation _returnvalue (Math|Rotator|MakeRotator 0.0 0.0 1.8e+02)))))

(event Custom|zombBackAndForth
  ;[0.8745 0.6314 1] Zombie Movement and Rotation Logic
  ;;[1 1 1] Move Back and forth based on timer
  (if (Variables|Default|GetisMoveRight)
    (CallFunction|ZombMoveRot 0.25)
    (else
      (CallFunction|ZombMoveRot -0.25)))
  (if (>= (- (Utilities|Time|GetGameTimeinSeconds) (Variables|Default|GetEnemyTime)) (Variables|Default|GetWhenRotate))
    (Variables|Default|SetisMoveRight (not (Variables|Default|GetisMoveRight)))
    (Variables|Default|SetEnemyTime (Math|Float|Truncate (Utilities|Time|GetGameTimeinSeconds)))))

(event EventBeginPlay
  (Variables|Default|SetEffect "/Game/BP/FX/Actor/PuffEffect.PuffEffect_C")
  (Variables|Default|SetEnemyTime (Math|Float|Truncate (Utilities|Time|GetGameTimeinSeconds)))
  (if (== (.yaw (Transformation|GetWorldRotation (Variables|Default|GetSprite))) 1.8e+02)
    (Variables|Default|SetisMoveRight true)
    (else
      (Variables|Default|SetisMoveRight false))))

(event EventTick
  (params (DeltaSeconds :type Float%20%28single-precision%29))
  (CallFunction|ZombBackandForth))

(fn ConstructionScript
  (|CallParentFunction))

(fn PuffEffect
  (bind _capsulecomponent (Variables|Default|GetCapsuleComponent))
  (bind _returnvalue (Transformation|GetWorldTransform _capsulecomponent))
  (Game|SpawnActorfromClass "/Game/BP/FX/Actor/PuffEffect.PuffEffect_C" (Math|Transform|MakeTransform (Math|Vector|MakeVector (.x (.location _returnvalue)) (+ (.y (.location _returnvalue)) 5.0) (.z (.location _returnvalue))) (.rotation _returnvalue) (.scale _returnvalue)) "Undefined" 0 0))
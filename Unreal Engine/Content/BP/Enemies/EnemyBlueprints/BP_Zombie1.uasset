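; BP_Zombie1 is an enemy zombie that patrols back and forth along the world X axis.
; Each tick it applies movement input, snaps controller yaw to face the travel direction, and increments a counter that flips direction every 150 ticks, so patrol timing depends on frame rate.
; Any actor overlap calls TakeDmg on the zombie itself, as temporary damage-test logic marked for removal.
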(event Custom|zombMoveRot
  (params (axisVal :type Float%20%28double-precision%29))
  (bind _returnvalue (Pawn|GetController))
  ;[0.8745 0.6314 1] Zombie Movement and Rotation Logic
  ;;[1 1 1] Movement + rotation for zombie
  (Pawn|Input|AddMovementInput "1.000000,0.000000, 0" axisVal false)
  (Math|Float|CompareFloat axisVal 0.0
    (:>
      (Pawn|SetControlRotation _returnvalue (Math|Rotator|MakeRotator 0.0 0.0 0.0)))
    (:<
      (Pawn|SetControlRotation _returnvalue (Math|Rotator|MakeRotator 0.0 0.0 1.8e+02)))))

(event Custom|zombBackAndForth
  ;[0.8745 0.6314 1] Zombie Movement and Rotation Logic
  ;;[1 1 1] Move Back and forth based on timer
  (if (Variables|Default|GetisMoveRight)
    (CallFunction|ZombMoveRot 1.0)
    (else
      (CallFunction|ZombMoveRot -1.0)))
  (bind _result (Math|Integer|IncrementInt (Variables|Default|GetzombTime))
    (:%20%20
      (bind _output_get (Variables|Default|SetzombTime _result))
      (if (== (Math|Integer|%(Integer) _output_get 150) 0)
        (Variables|Default|SetisMoveRight (not (Variables|Default|GetisMoveRight)))))))

(event EventTick
  (params (DeltaSeconds :type Float%20%28single-precision%29))
  (CallFunction|ZombBackandForth))

(event Collision|EventActorBeginOverlap
  (params (OtherActor :type Actor%20Object%20Reference))
  ;[1 1 1] Testing damage - Will delete later
  (CallFunction|TakeDmg 1e+01))

(fn ConstructionScript
  (|CallParentFunction))
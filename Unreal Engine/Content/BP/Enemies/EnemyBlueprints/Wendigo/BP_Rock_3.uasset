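; BP_Rock_3 is a rock projectile, filed with the Wendigo enemy, that damages the main character on hit.
; Overlapping the player's capsule with its Box calls Hurt with its DamageAmount, then destroys the rock.
; Otherwise it destroys itself when Tick sees its ProjectileMovement velocity at exactly zero, or ten seconds after spawning.
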(event OnComponentBeginOverlap(Box)
  (params (OverlappedComponent :type Primitive%20Component%20Object%20Reference) (OtherActor :type Actor%20Object%20Reference) (OtherComp :type Primitive%20Component%20Object%20Reference) (OtherBodyIndex :type Integer) (bFromSweep :type Boolean) (SweepResult :type Hit%20Result%20Structure%20%28by%20ref%29))
  ;[1 1 1] Determing and Hitting Enemies
  (bind _asbp_main_character (Utilities|Casting|CastToBP_MainCharacter OtherActor))
  (if (== (Variables|/Script/Engine.Character|GetCapsuleComponent _asbp_main_character) OtherComp)
    (Default|Hurt _asbp_main_character (Variables|Default|GetDamage%20Amount))
    (Actor|DestroyActor)))

(event EventBeginPlay
  ;[1 1 1] Destroy Projectile in 10 sec after spawn
  (Utilities|FlowControl|Delay 1e+01)
  (Actor|DestroyActor))

(event EventTick
  (params (DeltaSeconds :type Float%20%28single-precision%29))
  ;[1 1 1] If vlocity is 0 destroy projectile
  (if (Utilities|Operators|EqualEqual :A (Variables|/Script/Engine.MovementComponent|GetVelocity (Variables|Default|GetProjectileMovement)))
    (Actor|DestroyActor)))

(fn ConstructionScript)
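; BP_Rock_Trigger is a one-shot trigger volume that makes a Wendigo attack when its HitBox overlaps the Box.
; It calls the Wendigo's Attack and waits for the length of the sprite's flipbook.
; It then spawns two differently scaled actors at the Projectile component, with rotation derived from that component's world position, and destroys itself.
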(event OnComponentBeginOverlap(Box)
  (params (OverlappedComponent :type Primitive%20Component%20Object%20Reference) (OtherActor :type Actor%20Object%20Reference) (OtherComp :type Primitive%20Component%20Object%20Reference) (OtherBodyIndex :type Integer) (bFromSweep :type Boolean) (SweepResult :type Hit%20Result%20Structure%20%28by%20ref%29))
  (bind _projectile (Variables|Default|GetProjectile))
  (bind _returnvalue (Transformation|GetWorldLocation _projectile))
  (bind _returnvalue_2 (Math|Conversions|RotationFromXVector _returnvalue))
  ;[1 1 1] Determing and Hitting Enemies
  (bind _asbp_wendigo (Utilities|Casting|CastToBP_Wendigo OtherActor))
  (if (== (Variables|/Game/BP/Enemies/EnemyBlueprints/Wendigo/BP_Wendigo.BP_Wendigo_C|GetHitBox _asbp_wendigo) OtherComp)
    (Default|Attack _asbp_wendigo)
    (Utilities|FlowControl|Delay (Class|PaperFlipbookComponent|GetFlipbookLength (Variables|/Script/Paper2D.PaperCharacter|GetSprite _asbp_wendigo)))
    (Game|SpawnActorfromClass "/Game/BP/Enemies/EnemyBlueprints/Wendigo/BP_Rock_Wendigo.BP_Rock_Wendigo_C" (Math|Transform|MakeTransform _returnvalue _returnvalue_2 "2.500000,2.500000,2.500000") "Undefined" 0 0)
    (Game|SpawnActorfromClass "/Game/BP/FX/Actor/PuffEffect.PuffEffect_C" (Math|Transform|MakeTransform _returnvalue _returnvalue_2 "2.000000,2.000000,2.000000") "Undefined" 0 0)
    (Actor|DestroyActor)))

(fn ConstructionScript)
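; BP_Ogre is a 2D flipbook enemy that periodically throws rocks.
; Tick compares game time against WhenShoot, then switches CharState to throw, where State swaps the flipbook and spawns BP_Rock at the Projectile transform.
; A Delay matching the flipbook length returns CharState to idle and restarts the timer.
; It also defines a zombie-named X-axis move-and-turn event and a puff spawn function, and sets Effect on BeginPlay.
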(event Custom|State
  (switch int (Variables|Default|GetCharState)
    (:0
      (Sprite|SetFlipbook (Variables|Default|GetSprite) "/Game/BP/Enemies/AllEnemies/Ogre/Flipbooks/ogre-idle.ogre-idle"))
    (:1
      (Sprite|SetFlipbook (Variables|Default|GetSprite) "/Game/BP/Enemies/AllEnemies/Ogre/Flipbooks/ogre-throw.ogre-throw")
      (Game|SpawnActorfromClass "/Game/BP/Projectile/Ogre/BP_Rock.BP_Rock_C" (Transformation|GetWorldTransform (Variables|Default|GetProjectile)) "Undefined" 0 0))))

(event Custom|zombMoveRot
  (params (axisVal :type Float%20%28double-precision%29))
  (bind _returnvalue (Pawn|GetController))
  ;[0.8745 0.6314 1] Zombie Movement and Rotation Logic
  ;;[1 1 1] Movement + rotation for zombie
  (Pawn|Input|AddMovementInput "1.000000,0.000000, 0" axisVal false)
  (Math|Float|CompareFloat axisVal 0.0
    (:>
      (Pawn|SetControlRotation _returnvalue (Math|Rotator|MakeRotator 0.0 0.0 0.0)))
    (:<
      (Pawn|SetControlRotation _returnvalue (Math|Rotator|MakeRotator 0.0 0.0 1.8e+02)))))

(event EventBeginPlay
  (Variables|Default|SetEffect "/Game/BP/FX/Actor/PuffEffect.PuffEffect_C")
  (Variables|Default|SetEnemyTime (Math|Float|Truncate (Utilities|Time|GetGameTimeinSeconds))))

(event EventTick
  (params (DeltaSeconds :type Float%20%28single-precision%29))
  ;[0.8745 0.6314 1] Zombie Movement and Rotation Logic
  ;;[1 1 1] Projectile Attack
  (if (== (Variables|Default|GetCharState) 0)
    (CallFunction|State)
    (if (>= (- (Utilities|Time|GetGameTimeinSeconds) (Variables|Default|GetEnemyTime)) (Variables|Default|GetWhenShoot))
      (Variables|Default|SetCharState 1)
      (CallFunction|State)
      (Utilities|FlowControl|Delay (Class|PaperFlipbookComponent|GetFlipbookLength (Variables|Default|GetSprite)))
      (Variables|Default|SetCharState 0)
      (Variables|Default|SetEnemyTime (Math|Float|Truncate (Utilities|Time|GetGameTimeinSeconds))))))

(fn ConstructionScript
  (|CallParentFunction))

(fn PuffEffect
  (bind _capsulecomponent (Variables|Default|GetCapsuleComponent))
  (bind _returnvalue (Transformation|GetWorldTransform _capsulecomponent))
  (Game|SpawnActorfromClass "/Game/BP/FX/Actor/PuffEffect.PuffEffect_C" (Math|Transform|MakeTransform (Math|Vector|MakeVector (.x (.location _returnvalue)) (+ (.y (.location _returnvalue)) 5.0) (.z (.location _returnvalue))) (.rotation _returnvalue) (.scale _returnvalue)) "Undefined" 0 0))
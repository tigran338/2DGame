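; Paper2D Wendigo enemy that runs along +X and melees the main character, with a puff effect set up on BeginPlay.
; Tick polls HitBox overlap against the player's capsule to trigger Attack, and otherwise drives movement and the run flipbook.
; Attack waits out its flipbook, rechecks overlap before calling Hurt, then returns to idle.
; A zombie-derived move-and-rotate event and an empty State switch are also present, but nothing here calls them.
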(event Custom|State
  (switch int (Variables|Default|GetCharState)))

(event Custom|Attack
  (params (Actor :type BP%20Main%20Character%20Object%20Reference))
  (bind _sprite (Variables|Default|GetSprite))
  ;[1 1 1] Attack
  (Variables|Default|SetisAttack true)
  (Sprite|SetFlipbook _sprite "/Game/BP/Enemies/AllEnemies/Wendigo_Boss/Flipbook/wendigo_Atk.wendigo_Atk")
  (Utilities|FlowControl|Delay (Class|PaperFlipbookComponent|GetFlipbookLength _sprite))
  (bind _isableattack (CallFunction|IsAbleAttack))
  (if _isableattack
    (Default|Hurt Actor 0.01))
  (Sprite|SetFlipbook (Variables|Default|GetSprite) "/Game/BP/Enemies/AllEnemies/Wendigo_Boss/Flipbook/wendigo_Idle.wendigo_Idle")
  (Variables|Default|SetisAttack false))

(event Custom|zombMoveRot
  (params (axisVal :type Float%20%28double-precision%29))
  (bind _returnvalue (Pawn|GetController))
  ;[0.8745 0.6314 1] Zombie Movement and Rotation Logic
  ;;[1 1 1] Movement + rotation for zombie
  (Pawn|Input|AddMovementInput "1.000000,0.000000, 0" axisVal false)
  (Math|Float|CompareFloat axisVal 0.0
    (:>
      (Pawn|SetControlRotation _returnvalue (Math|Rotator|MakeRotator 0.0 0.0 0.0)))
    (:<
      (Pawn|SetControlRotation _returnvalue (Math|Rotator|MakeRotator 0.0 0.0 1.8e+02)))))

(event EventBeginPlay
  (Variables|Default|SetEffect "/Game/BP/FX/Actor/PuffEffect.PuffEffect_C")
  (Variables|Default|SetEnemyTime (Math|Float|Truncate (Utilities|Time|GetGameTimeinSeconds))))

(event EventTick
  (params (DeltaSeconds :type Float%20%28single-precision%29))
  ;[0.8745 0.6314 1] Zombie Movement and Rotation Logic
  ;;[1 1 1] Main
  (Utilities|FlowControl|Sequence
    (:then_0
      (bind (_isableattack _actor) (CallFunction|IsAbleAttack))
      (if _isableattack
        (CallFunction|Attack _actor)))
    (:then_1
      (if (not (Variables|Default|GetisAttack))
        (Pawn|Input|AddMovementInput "1.000000, 0, 0" 1.0 false)
        (Sprite|SetFlipbook (Variables|Default|GetSprite) "/Game/BP/Enemies/AllEnemies/Wendigo_Boss/Flipbook/wendigo_Run.wendigo_Run")))))

(fn ConstructionScript
  (|CallParentFunction))

(fn PuffEffect
  (bind _capsulecomponent (Variables|Default|GetCapsuleComponent))
  (bind _returnvalue (Transformation|GetWorldTransform _capsulecomponent))
  (Game|SpawnActorfromClass "/Game/BP/FX/Actor/PuffEffect.PuffEffect_C" (Math|Transform|MakeTransform (Math|Vector|MakeVector (.x (.location _returnvalue)) (+ (.y (.location _returnvalue)) 5.0) (.z (.location _returnvalue))) (.rotation _returnvalue) (.scale _returnvalue)) "Undefined" 0 0))

(fn IsAbleAttack
  (for _array_element (Collision|GetOverlappingActors (Variables|Default|GetHitBox) 0 :!class /Script/Engine.PrimitiveComponent)
    (bind _asbp_main_character (Utilities|Casting|CastToBP_MainCharacter _array_element))
    (return (and (Class|PrimitiveComponent|IsOverlappingComponent (Variables|Default|GetHitBox) (Variables|/Script/Engine.Character|GetCapsuleComponent _asbp_main_character)) (!= (Variables|Default|GetSprite) "/Game/BP/Enemies/AllEnemies/Wendigo_Boss/Flipbook/wendigo_Atk.wendigo_Atk")) _asbp_main_character))
  (return false 0))
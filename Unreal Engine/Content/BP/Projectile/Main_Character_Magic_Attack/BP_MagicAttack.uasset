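; BP_MagicAttack is the main character's magic attack projectile, moved by a projectile movement component.
; Its Box overlap applies DamageAmount through TakeDmg to BP_ENEMYINHERITABLE actors, only when their capsule component is hit, then destroys the projectile.
; It also destroys itself when Tick finds its velocity at zero, or after a fixed lifetime delay from BeginPlay.
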(event OnComponentBeginOverlap(Box)
  (params (OverlappedComponent :type Primitive%20Component%20Object%20Reference) (OtherActor :type Actor%20Object%20Reference) (OtherComp :type Primitive%20Component%20Object%20Reference) (OtherBodyIndex :type Integer) (bFromSweep :type Boolean) (SweepResult :type Hit%20Result%20Structure%20%28by%20ref%29))
  (bind _asbp_enemyinheritable (Utilities|Casting|CastToBP_ENEMYINHERITABLE OtherActor))
  (if (== (Variables|/Script/Engine.Character|GetCapsuleComponent _asbp_enemyinheritable) OtherComp)
    (Default|TakeDmg _asbp_enemyinheritable (Math|Conversions|ToFloat(Integer) (Variables|Default|GetDamage%20Amount)))
    (Actor|DestroyActor)))

(event EventBeginPlay
  (Utilities|FlowControl|Delay 1e+01)
  (Actor|DestroyActor))

(event EventTick
  (params (DeltaSeconds :type Float%20%28single-precision%29))
  (if (Utilities|Operators|EqualEqual :A (Variables|/Script/Engine.MovementComponent|GetVelocity (Variables|Default|GetProjectileMovement)))
    (Actor|DestroyActor)))

(fn ConstructionScript)
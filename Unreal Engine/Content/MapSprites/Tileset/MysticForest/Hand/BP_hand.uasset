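; BP_hand is a Mystic Forest map hazard, an animated hand that hurts the main character on contact.
; Each tick it checks the actors overlapping its Box and calls Hurt on any BP_MainCharacter whose capsule touches the box.
; On BeginPlay it sets the Hand animation to a random playback position so placed copies do not animate in sync.
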(event EventBeginPlay
  (Components|Timeline|SetPlaybackPosition (Variables|Default|Gethand) (Math|Random|RandomFloat) false))

(event Collision|EventActorBeginOverlap
  (params (OtherActor :type Actor%20Object%20Reference)))

(event EventTick
  (params (DeltaSeconds :type Float%20%28single-precision%29))
  (for _array_element (Collision|GetOverlappingActors (Variables|Default|GetBox) 0 :!class /Script/Engine.PrimitiveComponent)
    (bind _asbp_main_character (Utilities|Casting|CastToBP_MainCharacter _array_element))
    (if (Class|PrimitiveComponent|IsOverlappingComponent (Variables|Default|GetBox) (Variables|/Script/Engine.Character|GetCapsuleComponent _asbp_main_character))
      (Default|Hurt _asbp_main_character 1.0))))

(fn ConstructionScript)
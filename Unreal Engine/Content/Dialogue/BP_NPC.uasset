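; BP_NPC is a 2D NPC character Blueprint with an UpdateAnimation event meant to pick its sprite flipbook.
; A switch on CharState maps movement, attack, hurt and death states to matching flipbooks.
; That switch sits behind an airborne check and a hardcoded branch that never passes, so it cannot run as written.
; Nothing shown calls the event or sets the state, and the construction script is empty.
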(event Custom|Update%20Animation
  ;[0 1 0.1717] Upadte Animation
  (if (not (AI|Components|NavMovement|IsMovingonGround (Variables|Character|GetCharacterMovement)))
    (if (not true)
      (Utilities|FlowControl|Sequence
        (:then_3
          ;;[1 1 1] Turn on Animation
          (switch Utilities|FlowControl|Switch|SwitchonChar_State (Variables|Default|GetChar%20State)
            (:NewEnumerator0
              (Sprite|SetFlipbook (Variables|Default|GetSprite) "/Game/BP/Character/Animations/Flipbook/Idle.Idle"))
            (:NewEnumerator1
              (Sprite|SetFlipbook (Variables|Default|GetSprite) "/Game/BP/Character/Animations/Flipbook/Run.Run"))
            (:NewEnumerator2
              (Sprite|SetFlipbook (Variables|Default|GetSprite) "/Game/BP/Character/Animations/Flipbook/Jump.Jump"))
            (:NewEnumerator3
              (Sprite|SetFlipbook (Variables|Default|GetSprite) "/Game/BP/Character/Animations/Flipbook/Sword_Attack.Sword_Attack"))
            (:NewEnumerator4
              (Sprite|SetFlipbook (Variables|Default|GetSprite) "/Game/BP/Character/Animations/Flipbook/Jump_Attack.Jump_Attack"))
            (:NewEnumerator5
              (Sprite|SetFlipbook (Variables|Default|GetSprite) "/Game/BP/Character/Animations/Flipbook/Throw.Throw"))
            (:NewEnumerator6
              (Sprite|SetFlipbook (Variables|Default|GetSprite) "/Game/BP/Character/Animations/Flipbook/Hurt.Hurt"))
            (:NewEnumerator7
              (Sprite|SetFlipbook (Variables|Default|GetSprite) "/Game/BP/Character/Animations/Flipbook/Dead.Dead"))))))))

(fn ConstructionScript)
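; BP_HellBeast is an unfinished 2D flipbook enemy that detects the main character with a sphere trigger.
; Sphere overlap begin and end toggle FoundPC, and both set the idle flipbook.
; Each tick, while FoundPC is true, it compares its X position against the player's, but nothing follows the comparison.
; The attack event is empty, and the burn flipbook and 180-degree control-rotation nodes are disconnected.
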(event OnComponentBeginOverlap(SphereColl)
  (params (OverlappedComponent :type Primitive%20Component%20Object%20Reference) (OtherActor :type Actor%20Object%20Reference) (OtherComp :type Primitive%20Component%20Object%20Reference) (OtherBodyIndex :type Integer) (bFromSweep :type Boolean) (SweepResult :type Hit%20Result%20Structure%20%28by%20ref%29))
  ;[1 1 1] Set FoundPC if within Sphere
  (Utilities|Casting|CastToBP_MainCharacter OtherActor)
  (Variables|Default|SetfoundPC true)
  (Sprite|SetFlipbook (Variables|Default|GetSprite) "/Game/BP/Enemies/AllEnemies/HellBeast/Flipbooks/hell-beast-idle.hell-beast-idle"))

(event OnComponentEndOverlap(SphereColl)
  (params (OverlappedComponent :type Primitive%20Component%20Object%20Reference) (OtherActor :type Actor%20Object%20Reference) (OtherComp :type Primitive%20Component%20Object%20Reference) (OtherBodyIndex :type Integer))
  ;[1 1 1] Set FoundPC if within Sphere
  (Utilities|Casting|CastToBP_MainCharacter OtherActor)
  (Variables|Default|SetfoundPC false)
  (Sprite|SetFlipbook (Variables|Default|GetSprite) "/Game/BP/Enemies/AllEnemies/HellBeast/Flipbooks/hell-beast-idle.hell-beast-idle"))

(event Custom|hellBeastLookAtPC
  ;[1 1 1] Looking at PC if found
  (if (Variables|Default|GetfoundPC)
    (bind _asbp_main_character (Utilities|Casting|CastToBP_MainCharacter (Game|GetPlayerCharacter 0)))
    (Math|Float|CompareFloat (- (.x (Transformation|GetWorldLocation (Variables|Default|GetCapsuleComponent))) (.x (Transformation|GetWorldLocation (Variables|/Script/Engine.Actor|GetRootComponent _asbp_main_character)))) 0.0)))

(event Custom|hellBeastAtk)

(event EventBeginPlay)

(event Collision|EventActorBeginOverlap
  (params (OtherActor :type Actor%20Object%20Reference)))

(event EventTick
  (params (DeltaSeconds :type Float%20%28single-precision%29))
  (CallFunction|HellBeastLookatPC))

(fn ConstructionScript
  (|CallParentFunction))
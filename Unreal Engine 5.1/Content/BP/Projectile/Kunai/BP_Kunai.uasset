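; BP_Kunai is a Paper2D kunai projectile that hurts an enemy on hit and destroys itself after a fixed lifetime.
; When its box begins an overlap, it scans overlapping actors for a BP_Enemy whose capsule touches the box and calls Hurt on the first match.
; A helper then copies the kunai sprite onto that enemy's capsule at its world transform, so it appears stuck after the projectile is destroyed.
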(event OnComponentBeginOverlap(Box)
  (params (OverlappedComponent :type Primitive%20Component%20Object%20Reference) (OtherActor :type Actor%20Object%20Reference) (OtherComp :type Primitive%20Component%20Object%20Reference) (OtherBodyIndex :type Integer) (bFromSweep :type Boolean) (SweepResult :type Hit%20Result%20Structure%20%28by%20ref%29))
  (bind _box (Variables|Default|GetBox))
  (bind _box_2 (Variables|Default|GetBox))
  (Utilities|IsValid _box_2
    (:Is%20Valid
      (bind _array_element (Utilities|Array|ForEachLoopwithBreak (Collision|GetOverlappingActors _box_2 0 :!class /Script/Engine.PrimitiveComponent) :!label _label)
        (:LoopBody
          (bind _asbp_enemy (Utilities|Casting|CastToBP_Enemy _array_element))
          (Utilities|IsValid _box
            (:Is%20Valid
              (if (Class|PrimitiveComponent|IsOverlappingComponent _box (Variables|/Script/Engine.Character|GetCapsuleComponent _asbp_enemy))
                (Variables|Default|SetDestroy (Class|PrimitiveComponent|IsOverlappingComponent _box (Variables|/Script/Engine.Character|GetCapsuleComponent _asbp_enemy)))
                (Default|Hurt _asbp_enemy)
                (|AttachKunaitoEnemy _asbp_enemy (Variables|/Script/Engine.Character|GetCapsuleComponent _asbp_enemy))
                (goto _label Break)))))
        (:Completed
          (if (Variables|Default|GetDestroy)
            (Actor|DestroyActor)))))))

(event EventBeginPlay
  (Utilities|FlowControl|Delay 2e+01)
  (Actor|DestroyActor))

(event Collision|EventActorBeginOverlap
  (params (OtherActor :type Actor%20Object%20Reference)))

(fn ConstructionScript)